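; BP_SpaceShip is a pilotable physics spaceship that the player possesses on Enter, riding hidden at the Pilot socket, and leaves via Interact at the interaction trigger.
; Input axes apply pitch, yaw and roll torques, while Thrust eases a throttle value.
; The TakeOff axis drives a mass- and tilt-compensated lift thruster at low throttle, switching to direct forward velocity above a threshold.
; BeginPlay aligns the center of mass with the thruster.
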(event `InputAction|Interact`
  (params (Key :type "Key Structure"))
  (:`Pressed`
    (`self.Exit`)))

(event `InputAxis|TakeOff`
  (params (AxisValue :type "Float (single-precision)"))
  (bind (_returnvalue_x _returnvalue_y _returnvalue_z) (`KismetMathLibrary.BreakVector` (`self.GetActorUpVector`)))
  (if (>= (`self.Thurst`) 100.0)
    (`PrimitiveComponent.SetPhysicsLinearVelocity` (`self.SpaceShip`) (`self.ForwardVelocity`) false "None")
    (else
      (set `PhysicsThrusterComponent.ThrustStrength` (* (/ (* AxisValue 500.0) _returnvalue_z) (`PrimitiveComponent.GetMass` (`self.SpaceShip`))) (`self.PhysicsThruster`)))))

(event `self.ReceiveBeginPlay`
  (bind (_returnvalue_x _returnvalue_y) (`KismetMathLibrary.BreakVector` (`KismetMathLibrary.GreaterGreater_VectorRotator` (- (`SceneComponent.K2_GetComponentLocation` (`self.PhysicsThruster`)) (`PrimitiveComponent.GetCenterOfMass` (`self.SpaceShip`) "None")) (`KismetMathLibrary.NegateRotator` (`SceneComponent.K2_GetComponentRotation` (`self.SpaceShip`))))))
  (`PrimitiveComponent.SetCenterOfMass` (`self.SpaceShip`) (`KismetMathLibrary.MakeVector` _returnvalue_x _returnvalue_y) "None"))

(event `InputAxis|MoveUp`
  (params (AxisValue :type "Float (single-precision)"))
  (`PrimitiveComponent.AddTorqueInDegrees` (`self.SpaceShip`) (* (`SceneComponent.GetRightVector` (`self.SpaceShip`)) (* AxisValue (`self.ForwardTorquePower`))) "None" true))

(event `InputAxis|MoveRight`
  (params (AxisValue :type "Float (single-precision)"))
  (`PrimitiveComponent.AddTorqueInDegrees` (`self.SpaceShip`) (* (`SceneComponent.GetUpVector` (`self.SpaceShip`)) (* AxisValue (`self.SideTorquePower`))) "None" true))

(event `InputAxis|Roll`
  (params (AxisValue :type "Float (single-precision)"))
  (`PrimitiveComponent.AddTorqueInDegrees` (`self.SpaceShip`) (* (`SceneComponent.GetForwardVector` (`self.SpaceShip`)) (* AxisValue (`self.RotateTorque`))) "None" true))

(event `InputAxis|Thrust`
  (params (AxisValue :type "Float (single-precision)"))
  (`|ExecutionSequence`
    (:`then_0`
      (if (not (`KismetMathLibrary.NearlyEqual_FloatFloat` AxisValue 0.0 0.1))
        (set `self.Thurst` (`KismetMathLibrary.FInterpTo` (`self.Thurst`) (`KismetMathLibrary.Lerp` 0.0 (`self.MaxThurst`) (/ (+ AxisValue 1.0) 2.0)) (`GameplayStatics.GetWorldDeltaSeconds`) 1.0))))
    (:`then_1`
      (set `self.ForwardVelocity` (* (`SceneComponent.GetForwardVector` (`self.SpaceShip`)) (`self.Thurst`))))))

(fn `Enter`
  (params (Player :type "/Game/ThirdPerson/Blueprints/BP_ThirdPersonCharacter Object Reference") (ExitDelegate :type "Delegate (by ref)"))
  (add `self.OnExited` ExitDelegate)
  (bind _output_get (set `self.PlayerRef` Player))
  (`Controller.Possess` (`self.GetController` _output_get) self)
  (`self.K2_AttachToActor` (`self.PlayerRef`) self "Pilot" "SnapToTarget" "SnapToTarget" "SnapToTarget" true)
  (`/Game/ThirdPerson/Blueprints/BP_ThirdPersonCharacter.HidePlayer` (`self.PlayerRef`)))

(fn `Exit`
  (`self.K2_DetachFromActor` (`self.PlayerRef`) "KeepWorld" "KeepWorld" "KeepWorld")
  (`self.K2_SetActorLocation` (`self.PlayerRef`) (`SceneComponent.GetSocketLocation` (`self.InteractionTrigger`) "None") false false)
  (`Controller.Possess` (`self.GetController`) (`self.PlayerRef`))
  (`/Game/ThirdPerson/Blueprints/BP_ThirdPersonCharacter.UnhidePlayer` (`self.PlayerRef`))
  (`self.OnExited`))

(fn `UserConstructionScript`)